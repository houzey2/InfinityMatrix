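; BP_Enemy is an enemy actor that resolves everything on its Enemy component's begin-overlap event and destroys itself on contact.
; Hitting BP_Player subtracts health, updates the HUD bar, plays a camera shake, shows a WBP_Hurt widget, and calls DisplayRestart once health runs out.
; Any other overlapping actor, not only bullets, awards the player score and destroys the enemy; the bullet-destroy nodes are never executed.
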(event `self.enemy.OnComponentBeginOverlap`
  (params (OverlappedComponent :type "PrimitiveComponent Object Reference") (OtherActor :type "Actor Object Reference") (OtherComp :type "PrimitiveComponent Object Reference") (OtherBodyIndex :type Integer) (bFromSweep :type Boolean) (SweepResult :type "HitResult Structure (by ref)"))
  (bind _asbp_player (cast `/Game/InfiniteMatrix/Blueprints/BP_Player` OtherActor)
    (:`then`
      (bind _health (`/Game/InfiniteMatrix/Blueprints/BP_Player.Health` _asbp_player))
      (if (> _health 0)
        (bind _output_get (set `/Game/InfiniteMatrix/Blueprints/BP_Player.Health` (- _health 10) _asbp_player))
        (`/Game/InfiniteMatrix/UI/WBP_HUD.UpdateHealthBar` (`/Game/InfiniteMatrix/Blueprints/BP_Player.WB_HUD` _asbp_player) (`KismetMathLibrary.Conv_IntToDouble` _output_get)))
      (`GameplayStatics.PlayWorldCameraShake` "/Game/InfiniteMatrix/Blueprints/Shake.Shake_C" (`self.K2_GetActorLocation` _asbp_player) 0.0 500.0)
      (`self.K2_DestroyActor`)
      (bind _returnvalue (`|CreateWidget` "/Game/InfiniteMatrix/UI/WBP_Hurt.WBP_Hurt_C"))
      (`UserWidget.AddToViewport` _returnvalue 0)
      (if (<= (`/Game/InfiniteMatrix/Blueprints/BP_Player.Health` _asbp_player) 0)
        (bind _asbp_player_2 (cast `/Game/InfiniteMatrix/Blueprints/BP_Player` (`GameplayStatics.GetPlayerPawn` 0)))
        (`/Game/InfiniteMatrix/Blueprints/BP_Player.Display Restart` _asbp_player_2)))
    (:`CastFailed`
      (bind _asbp_player_3 (cast `/Game/InfiniteMatrix/Blueprints/BP_Player` (`GameplayStatics.GetPlayerPawn` 0))
        (:`then`
          (set `/Game/InfiniteMatrix/Blueprints/BP_Player.Score` (+ (`/Game/InfiniteMatrix/Blueprints/BP_Player.Score` _asbp_player_3) 50) _asbp_player_3))
        (:`CastFailed`
          _))
      (`self.K2_DestroyActor`))))

(fn `UserConstructionScript`)